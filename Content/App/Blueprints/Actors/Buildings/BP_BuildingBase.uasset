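; Base actor for city buildings that outlines on hover and opens its menu when clicked.
; Hover toggles custom depth, limited to the placed building during placement; construction applies the PlayerState's building material.
; Clicks are blocked during placement or tutorial, except farm and market when Flag1 is set.
; The recruitment, resource or standard widget receives BuildingID and takes UI-only input; recruitment also advances the tutorial for new players.
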(event Custom|OnClicked_Event
  (params (TouchedActor :type Actor%20Object%20Reference) (ButtonPressed :type Key%20Structure :default "None"))
  (CallFunction|HandleBuildingWidget))

(event MouseInput|EventActorEndCursorOver
  (CallFunction|HandleBuildingHover false))

(event MouseInput|EventActorBeginCursorOver
  (CallFunction|HandleBuildingHover true))

(event EventBeginPlay
  (EventDispatchers|BindEventtoOnClicked (delegate Custom|OnClicked_Event)))

(fn ConstructionScript
  (CallFunction|HandleBuildingMaterial))

(fn HandleBuildingHover
  (params (IsOutlining :type Boolean))
  (if (not IsOutlining)
    (Rendering|SetRenderCustomDepth (Variables|Default|GetBuildingMesh) false)
    (return)
    (else
      (Rendering|SetRenderCustomDepth (Variables|Default|GetBuildingMesh) (or (not (Variables|/Game/App/Blueprints/Utilities/BP_PlayerState.BP_PlayerState_C|GetIsPlacing (.AsBP%20Player%20State (Utilities|Casting|CastToBP_PlayerState (Game|GetPlayerState 0))))) (Variables|Default|GetBeingPlaced)))
      (return))))

(fn HandleBuildingWidget
  (bind _returnvalue (Game|GetPlayerState 0))
  (bind _buildingdata (Variables|Default|GetBuildingData))
  (bind _asbp_player_state (Utilities|Casting|CastToBP_PlayerState _returnvalue))
  (if (or (and (not (Variables|/Game/App/Blueprints/Utilities/BP_PlayerState.BP_PlayerState_C|GetIsPlacing _asbp_player_state)) (not (Variables|/Game/App/Blueprints/Utilities/BP_PlayerState.BP_PlayerState_C|GetIsNew _asbp_player_state))) (and (or (Utilities|Enum|Equal(Enum) (.name _buildingdata) "farm") (Utilities|Enum|Equal(Enum) (.name _buildingdata) "market")) (Variables|/Game/App/Blueprints/Utilities/BP_PlayerState.BP_PlayerState_C|GetFlag1 _asbp_player_state)))
    (bind _returnvalue_2 (UserInterface|CreateWidget (Variables|Default|GetWidgetClass) (Game|GetPlayerController 0)))
    (LocalVariables|SetBuildingWidget _returnvalue_2)
    (if (not (.bSuccess (Utilities|Casting|CastToWBP_Recruitment (LocalVariables|GetBuildingWidget))))
      (if (not (.bSuccess (Utilities|Casting|CastToWBP_Resource (LocalVariables|GetBuildingWidget))))
        (if (not (.bSuccess (Utilities|Casting|CastToWBP_Standard (LocalVariables|GetBuildingWidget))))
          (return)
          (else
            (Variables|/Game/App/Blueprints/Widgets/Board/Modals/WBP_Standard.WBP_Standard_C|SetBuildingID (.AsWBP%20Standard (Utilities|Casting|CastToWBP_Standard (LocalVariables|GetBuildingWidget))) (Variables|Default|GetBuildingID))
            (Default|HandleWidgetData (.AsWBP%20Standard (Utilities|Casting|CastToWBP_Standard (LocalVariables|GetBuildingWidget))))
            (UserInterface|Viewport|AddtoViewport (LocalVariables|GetBuildingWidget) 0)
            (Input|SetInputModeUIOnly (Game|GetPlayerController 0) 0 "DoNotLock" false)
            (return)))
        (else
          (Variables|/Game/App/Blueprints/Widgets/Board/Modals/WBP_Resource.WBP_Resource_C|SetBuildingID (.AsWBP%20Resource (Utilities|Casting|CastToWBP_Resource (LocalVariables|GetBuildingWidget))) (Variables|Default|GetBuildingID))
          (Default|HandleWidgetData (.AsWBP%20Resource (Utilities|Casting|CastToWBP_Resource (LocalVariables|GetBuildingWidget))))
          (UserInterface|Viewport|AddtoViewport (LocalVariables|GetBuildingWidget) 0)
          (Input|SetInputModeUIOnly (Game|GetPlayerController 0) 0 "DoNotLock" false)
          (return)))
      (else
        (Variables|/Game/App/Blueprints/Widgets/Board/Modals/WBP_Recruitment.WBP_Recruitment_C|SetBuildingID (.AsWBP%20Recruitment (Utilities|Casting|CastToWBP_Recruitment (LocalVariables|GetBuildingWidget))) (Variables|Default|GetBuildingID))
        (Default|HandleWidgetData (.AsWBP%20Recruitment (Utilities|Casting|CastToWBP_Recruitment (LocalVariables|GetBuildingWidget))))
        (UserInterface|Viewport|AddtoViewport (LocalVariables|GetBuildingWidget) 0)
        (Input|SetInputModeUIOnly (Game|GetPlayerController 0) 0 "DoNotLock" false)
        (if (Variables|/Game/App/Blueprints/Utilities/BP_PlayerState.BP_PlayerState_C|GetIsNew (.AsBP%20Player%20State (Utilities|Casting|CastToBP_PlayerState (Game|GetPlayerState 0))))
          (CallFunction|HandleTutorialLogic)
          (else
            (return)))))
    (else
      (return))))

(fn HandleBuildingMaterial
  (Rendering|Material|SetMaterial (Variables|Default|GetBuildingMesh) 0 (Variables|/Game/App/Blueprints/Utilities/BP_PlayerState.BP_PlayerState_C|GetBuildingMaterial (.AsBP%20Player%20State (Utilities|Casting|CastToBP_PlayerState (Game|GetPlayerState 0)))))
  (return))

(fn HandleTutorialLogic
  (Variables|/Game/App/Blueprints/Controllers/PlayerControllers/BP_CityBoardController.BP_CityBoardController_C|GetControllerActiveWidget (.AsBP%20City%20Board%20Controller (Utilities|Casting|CastToBP_CityBoardController (Game|GetPlayerController 0)))
    (:then
      (if (Variables|/Game/App/Blueprints/Utilities/BP_PlayerState.BP_PlayerState_C|GetFlag1 (.AsBP%20Player%20State (Utilities|Casting|CastToBP_PlayerState (Game|GetPlayerState 0))))
        (Default|Recruit (.AsWBP%20Introduction (Utilities|Casting|CastToWBP_Introduction (Variables|Default|GetController%20Active%20Widget))))))
    (:else)))