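; BP_Housing is the Housing building actor, a child building that represents level 1 housing with a Peasant unit image.
; The construction script runs the parent's, then assigns WBP_Standard as its widget class and fills in its building data.
; On BeginPlay it scans the player state's BuildingData values for entries named "Housing" and stores the last matching loop index as HouseNumber, a position among all buildings rather than a count of houses.
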(event EventBeginPlay
  (|CallParentFunction)
  (bind _values (Utilities|Map|Values (Variables|/Game/App/Blueprints/Utilities/BP_PlayerState.BP_PlayerState_C|GetBuildingData (.AsBP%20Player%20State (Utilities|Casting|CastToBP_PlayerState (Game|GetPlayerState 0))))))
  (for _array_element _values
    (if (Utilities|Enum|Equal(Enum) (.name _array_element) "Housing")
      (Variables|Default|SetIndex (Variables|Default|GetIndex))))
  (Variables|Default|SetHouseNumber (Variables|Default|GetIndex)))

(fn ConstructionScript
  (|CallParentFunction)
  (Variables|Default|SetWidgetClass "/Game/App/Blueprints/Widgets/Board/Modals/WBP_Standard.WBP_Standard_C")
  (Variables|Default|SetBuildingData (Utilities|Struct|MakeBuildingData "Housing" 1 "/Game/App/Blueprints/Widgets/Board/Assets/Peasant.Peasant")))