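; BP_Ploppable is a component that shows whether its owning actor's placement is valid through an outline post-process material.
; On BeginPlay and on every owner overlap begin or end, it treats placement as valid only when no actors overlap.
; It then swaps in the valid or invalid outline by overwriting PostProcessVolume settings, so the change is global rather than per mesh.
; The owner's cached static meshes only drive the loop that triggers the swap.
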(event Custom|OverlapStateChanged
  (params (OverlappedActor :type Actor%20Object%20Reference) (OtherActor :type Actor%20Object%20Reference))
  (CallFunction|HandleState))

(event EventBeginPlay
  (CallFunction|SetStaticMeshes)
  (Collision|BindEventtoOnActorBeginOverlap (Components|GetOwner) (delegate Custom|OverlapStateChanged))
  (Collision|BindEventtoOnActorEndOverlap (Components|GetOwner) (delegate Custom|OverlapStateChanged))
  (CallFunction|HandleState))

(fn HandleState
  (Variables|Default|SetIsPlacementValid (== (Utilities|Array|Length (Collision|GetOverlappingActors (Components|GetOwner) "/Script/Engine.Actor" :!class /Script/Engine.Actor)) 0))
  (for _array_element (Variables|Default|GetStaticMeshes)
    (LocalVariables|SetMesh _array_element)
    (if (Variables|Default|GetIsPlacementValid)
      (CallFunction|HandlePostProcessMaterialSwitch "/Game/App/Blueprints/Materials/MI_ValidOutline.MI_ValidOutline")
      (else
        (CallFunction|HandlePostProcessMaterialSwitch "/Game/App/Blueprints/Materials/MI_InvalidOutline.MI_InvalidOutline")))
    (return))
  (return))

(fn SetStaticMeshes
  (Variables|Default|SetStaticMeshes (Actor|GetComponentsByClass (Components|GetOwner) "/Script/Engine.StaticMeshComponent")))

(fn HandlePostProcessMaterialSwitch
  (params (Material :type Material%20Interface%20Object%20Reference))
  (bind _outactors (Actor|GetAllActorsOfClass "/Script/Engine.PostProcessVolume"))
  (for _array_element _outactors
    (bind _aspost_process_volume (Utilities|Casting|CastToPostProcessVolume _array_element))
    (Variables|/Script/Engine.PostProcessVolume|SetSettings _aspost_process_volume (Utilities|Struct|MakePostProcessSettings (Utilities|Struct|MakeWeightedBlendables (Utilities|Array|MakeArray (Utilities|Struct|MakeWeightedBlendable 1.0 Material)))))
    (return)))