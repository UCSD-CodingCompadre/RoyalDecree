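; Player controller for the city board that pans the pawn and handles mouse-driven building placement.
; Placement mode spawns a ploppable preview that follows a cursor line trace each tick and swaps the post-process outline material.
; Placing on a valid spot spawns the building, ends placement mode and, for new players, advances the introduction tutorial by checkpoint.
; The place input then records the last placed building's data and ID in the player state.
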(event Input|EnhancedActionEvents|EnhancedInputActionIA_MoveCamera
  (params (ActionValue :type Vector%202D%20Structure) (ElapsedSeconds :type Float%20%28double-precision%29) (TriggeredSeconds :type Float%20%28double-precision%29) (InputAction :type Input%20Action%20Object%20Reference :default "/Game/App/Blueprints/Input/IA_MoveCamera.IA_MoveCamera"))
  (Transformation|SetActorLocation (Variables|Default|GetPlayerPawn) (+ (* (Math|Vector|MakeVector (.y ActionValue) (.x ActionValue) 0.0) 25.0) (Transformation|GetActorLocation (Variables|Default|GetPlayerPawn))) false false))

(event Input|EnhancedActionEvents|EnhancedInputActionIA_PlaceBuilding
  (params (ActionValue :type Boolean) (ElapsedSeconds :type Float%20%28double-precision%29) (TriggeredSeconds :type Float%20%28double-precision%29) (InputAction :type Input%20Action%20Object%20Reference :default "/Game/App/Blueprints/Input/IA_PlaceBuilding.IA_PlaceBuilding"))
  (:Started
    (if (Variables|/Game/App/Blueprints/Utilities/BP_PlayerState.BP_PlayerState_C|GetIsPlacing (Variables|Default|GetCityBoardState))
      (CallFunction|SpawnBuilding)
      (CallFunction|UpdateBuildingData))))

(event EventBeginPlay
  (Input|AddMappingContext (PlayerController|LocalPlayerSubsystems|GetEnhancedInputLocalPlayerSubsystem) "/Game/App/Blueprints/Input/IMC_BoardPawn.IMC_BoardPawn" 0 "(bIgnoreAllPressedKeysUntilRelease=True,bForceImmediately=False,bNotifyUserSettings=False)")
  (Variables|Default|SetPlayerPawn (Game|Player|GetPlayerPawn 0))
  (CallFunction|HandleMouseSetup)
  (Variables|Default|SetCityBoardState (.AsBP%20Player%20State (Utilities|Casting|CastToBP_PlayerState (Game|GetPlayerState 0)))))

(event EventTick
  (params (DeltaSeconds :type Float%20%28single-precision%29))
  (if (Variables|Default|GetPlacementModeEnabled)
    (CallFunction|SetPlacement)))

(fn ConstructionScript)

(fn SetPlacementMode
  (params (SettingToEnable :type Boolean))
  (if (== SettingToEnable (Variables|Default|GetPlacementModeEnabled))
    (return)
    (else
      (bind _output_get (Variables|Default|SetPlacementModeEnabled SettingToEnable))
      (if _output_get
        (bind _returnvalue (Game|SpawnActorfromClass (Variables|Default|GetPlaceableActorType) (Math|Transform|MakeTransform "0.000000,0.000000,-100000.000000") "Undefined" "MultiplyWithRoot" 0 0))
        (bind _output_get_2 (Variables|Default|SetPlaceableActor _returnvalue))
        (AddComponent|AddBPPloppable _output_get_2)
        (Variables|/Game/App/Blueprints/Utilities/BP_PlayerState.BP_PlayerState_C|SetIsPlacing (.AsBP%20Player%20State (Utilities|Casting|CastToBP_PlayerState (Game|GetPlayerState 0))) true)
        (CallFunction|HandlePostProcessMaterialSwitch "/Game/App/Blueprints/Materials/MI_ValidOutline.MI_ValidOutline")
        (Variables|/Game/App/Blueprints/Actors/Buildings/BP_BuildingBase.BP_BuildingBase_C|SetBeingPlaced (.AsBP%20Building%20Base (Utilities|Casting|CastToBP_BuildingBase (Variables|Default|GetPlaceableActor))) true)
        (return)
        (else
          (bind _placeableactor (Variables|Default|GetPlaceableActor)
            (:then
              (Actor|DestroyActor _placeableactor))
            (:else)))))))

(fn SetPlacement
  (bind (_worldlocation _worlddirection) (Game|Player|ConvertMouseLocationToWorldSpace))
  (bind _outhit (Collision|LineTraceByChannel _worldlocation (+ _worldlocation (* _worlddirection 1e+04)) "TraceTypeQuery3" false 0 "None"))
  (if (.bBlockingHit (Collision|BreakHitResult _outhit))
    (bind _placeableactor (Variables|Default|GetPlaceableActor)
      (:then
        (Transformation|SetActorLocation _placeableactor (.Location (Collision|BreakHitResult _outhit)) false false)
        (return))
      (:else))))

(fn SpawnBuilding
  (bind _placeableactor (Variables|Default|GetPlaceableActor)
    (:then
      (Utilities|IsValid (Actor|GetComponentbyClass _placeableactor "/Game/App/Blueprints/Components/BP_Ploppable.BP_Ploppable_C")
        (:Is%20Valid
          (if (Variables|/Game/App/Blueprints/Components/BP_Ploppable.BP_Ploppable_C|GetIsPlacementValid (Actor|GetComponentbyClass _placeableactor "/Game/App/Blueprints/Components/BP_Ploppable.BP_Ploppable_C"))
            (bind _returnvalue (Game|SpawnActorfromClass (Variables|Default|GetPlaceableActorType) (Transformation|GetActorTransform (Variables|Default|GetPlaceableActor)) "AlwaysSpawn" "MultiplyWithRoot" 0 0))
            (Variables|Default|SetLastPlacedBuilding _returnvalue)
            (CallFunction|SetPlacementMode false)
            (Variables|/Game/App/Blueprints/Utilities/BP_PlayerState.BP_PlayerState_C|SetIsPlacing (.AsBP%20Player%20State (Utilities|Casting|CastToBP_PlayerState (Game|GetPlayerState 0))) false)
            (if (Variables|/Game/App/Blueprints/Utilities/BP_PlayerState.BP_PlayerState_C|GetIsNew (.AsBP%20Player%20State (Utilities|Casting|CastToBP_PlayerState (Game|GetPlayerState 0))))
              (bind _activewidget (Variables|Default|GetActiveWidget)
                (:then
                  (bind _aswbp_introduction (Utilities|Casting|CastToWBP_Introduction _activewidget))
                  (LocalVariables|SetIntroductionWidget _aswbp_introduction)
                  (CallFunction|HandlePostProcessMaterialSwitch "/Game/App/Blueprints/Materials/MI_BuildingOutline.MI_BuildingOutline")
                  ;[1 1 1] Tutorial Events
                  (switch int (Variables|/Game/App/Blueprints/Widgets/Board/Modals/WBP_Introduction.WBP_Introduction_C|GetCheckpoint (LocalVariables|GetIntroductionWidget))
                    (:Default
                      (return))
                    (:0
                      (Default|GameInfoStart (LocalVariables|GetIntroductionWidget)))
                    (:1
                      (Default|GameInfoContinue (LocalVariables|GetIntroductionWidget)))
                    (:2
                      (Default|GameInfoDone (LocalVariables|GetIntroductionWidget)))
                    (:3
                      (Default|UnitTutorialStart (LocalVariables|GetIntroductionWidget)))
                    (:4
                      (Default|PlaceRange (LocalVariables|GetIntroductionWidget)))
                    (:5
                      (Default|StartRecruiting (LocalVariables|GetIntroductionWidget))))
                  (return))
                (:else))
              (else
                (return)))))))
    (:else)))

(fn HandleMouseSetup
  (Variables|Default|SetbShowMouseCursor true)
  (Variables|Default|SetbEnableMouseOverEvents true)
  (Variables|Default|SetbEnableClickEvents true))

(fn HandlePostProcessMaterialSwitch
  (params (Material :type Material%20Interface%20Object%20Reference))
  (bind _outactors (Actor|GetAllActorsOfClass "/Script/Engine.PostProcessVolume"))
  (for _array_element _outactors
    (bind _aspost_process_volume (Utilities|Casting|CastToPostProcessVolume _array_element))
    (Variables|/Script/Engine.PostProcessVolume|SetSettings _aspost_process_volume (Utilities|Struct|MakePostProcessSettings (Utilities|Struct|MakeWeightedBlendables (Utilities|Array|MakeArray (Utilities|Struct|MakeWeightedBlendable 1.0 Material)))))
    (return)))

(fn UpdateBuildingData
  (LocalVariables|SetNewKey (Utilities|Map|Length (Variables|/Game/App/Blueprints/Utilities/BP_PlayerState.BP_PlayerState_C|GetBuildingData (Variables|Default|GetCityBoardState))))
  (Utilities|Map|Add (Variables|/Game/App/Blueprints/Utilities/BP_PlayerState.BP_PlayerState_C|GetBuildingData (Variables|Default|GetCityBoardState)) (LocalVariables|GetNewKey) (Variables|/Game/App/Blueprints/Actors/Buildings/BP_BuildingBase.BP_BuildingBase_C|GetBuildingData (.AsBP%20Building%20Base (Utilities|Casting|CastToBP_BuildingBase (Variables|Default|GetLastPlacedBuilding)))))
  (Variables|/Game/App/Blueprints/Actors/Buildings/BP_BuildingBase.BP_BuildingBase_C|SetBuildingID (.AsBP%20Building%20Base (Utilities|Casting|CastToBP_BuildingBase (Variables|Default|GetLastPlacedBuilding))) (LocalVariables|GetNewKey))
  (return))