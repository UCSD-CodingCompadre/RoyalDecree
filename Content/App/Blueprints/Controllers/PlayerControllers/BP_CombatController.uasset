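; BP_CombatController is the combat player controller, handling camera movement for a board pawn.
; On begin play it adds the board pawn input mapping context, caches the player pawn and enables the mouse cursor with click and hover events.
; The camera move action offsets the pawn location on X and Y by a fixed step per trigger, swapping input axes, without sweep or delta-time scaling.
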(event Input|EnhancedActionEvents|EnhancedInputActionIA_MoveCamera
  (params (ActionValue :type Vector%202D%20Structure) (ElapsedSeconds :type Float%20%28double-precision%29) (TriggeredSeconds :type Float%20%28double-precision%29) (InputAction :type Input%20Action%20Object%20Reference :default "/Game/App/Blueprints/Input/IA_MoveCamera.IA_MoveCamera"))
  (Transformation|SetActorLocation (Variables|Default|GetPlayerPawn) (+ (* (Math|Vector|MakeVector (.y ActionValue) (.x ActionValue) 0.0) 5.0) (Transformation|GetActorLocation (Variables|Default|GetPlayerPawn))) false false))

(event EventBeginPlay
  (Input|AddMappingContext (PlayerController|LocalPlayerSubsystems|GetEnhancedInputLocalPlayerSubsystem) "/Game/App/Blueprints/Input/IMC_BoardPawn.IMC_BoardPawn" 0 "(bIgnoreAllPressedKeysUntilRelease=True,bForceImmediately=False,bNotifyUserSettings=False)")
  (Variables|Default|SetPlayerPawn (Game|Player|GetPlayerPawn 0))
  (Variables|Default|SetbShowMouseCursor true)
  (Variables|Default|SetbEnableMouseOverEvents true)
  (Variables|Default|SetbEnableClickEvents true))

(fn ConstructionScript)